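; BP_figur is an animated figure actor whose legs, arms and head swing procedurally, without animation assets.
; Each Tick passes through a Gate, toggled by UI-facing open/close events, then steps each part's world rotation, reversing past ±20 degrees (roll for limbs, yaw for head).
; BeginPlay sets opposing start directions; slider events set head and per-arm speeds, while legs share Speed.
; The leg direction flags drive the opposite-named leg components.
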(event `self.ReceiveTick`
  (params (DeltaSeconds :type "Float (single-precision)"))
  (bind _rootrightleg (`self.RootRightLeg`))
  (bind _rootleftleg (`self.RootLeftLeg`))
  (bind _head (`self.Head`))
  (bind _rootrightarm (`self.RootRightArm`))
  (bind _rootleftarm (`self.RootLeftArm`))
  (bind (_returnvalue_roll _returnvalue_pitch _returnvalue_yaw) (`KismetMathLibrary.BreakRotator` (`SceneComponent.K2_GetComponentRotation` _rootrightleg)))
  (bind (_returnvalue_roll_2 _returnvalue_pitch_2 _returnvalue_yaw_2) (`KismetMathLibrary.BreakRotator` (`SceneComponent.K2_GetComponentRotation` _rootleftleg)))
  (bind (_returnvalue_roll_3 _returnvalue_pitch_3 _returnvalue_yaw_3) (`KismetMathLibrary.BreakRotator` (`SceneComponent.K2_GetComponentRotation` _rootleftarm)))
  (bind (_returnvalue_roll_4 _returnvalue_pitch_4 _returnvalue_yaw_4) (`KismetMathLibrary.BreakRotator` (`SceneComponent.K2_GetComponentRotation` _rootrightarm)))
  (bind (_returnvalue_roll_5 _returnvalue_pitch_5 _returnvalue_yaw_5) (`KismetMathLibrary.BreakRotator` (`SceneComponent.K2_GetComponentRotation` _head)))
  ;[1 1 1] EventTick: Gate can be accessed via Events (In the actual case our UI) to stop/continue the animation - Rotates limbs
  (`/Engine/EditorBlueprintResources/StandardMacros.Gate` false :!label _label
    (:`Exit`
      (`|ExecutionSequence`
        (:`then_0`
          ;[1 1 1] LeftLeg Movement
          ;;[1 1 1] Checks if it should rotate forward or backwards
          (if (`self.ForwardLeftLeg`)
            ;;[1 1 1] Checks if the rotation is greater than 20
            (if (> _returnvalue_roll 20.0)
              ;;[1 1 1] Either switches direction or sets a new rotation
              (set `self.ForwardLeftLeg` false)
              (else
                (`SceneComponent.K2_SetWorldRotation` _rootrightleg (`KismetMathLibrary.MakeRotator` (+ _returnvalue_roll (`self.Speed`)) _returnvalue_pitch _returnvalue_yaw) false false)))
            (else
              ;;[1 1 1] Checks if the rotation is less than -20
              (if (< _returnvalue_roll -20.0)
                (set `self.ForwardLeftLeg` true)
                (else
                  (`SceneComponent.K2_SetWorldRotation` _rootrightleg (`KismetMathLibrary.MakeRotator` (- _returnvalue_roll (`self.Speed`)) _returnvalue_pitch _returnvalue_yaw) false false))))))
        (:`then_1`
          ;[1 1 1] RightLeg Movement
          (if (`self.ForwardRightLeg`)
            (if (> _returnvalue_roll_2 20.0)
              (set `self.ForwardRightLeg` false)
              (else
                (`SceneComponent.K2_SetWorldRotation` _rootleftleg (`KismetMathLibrary.MakeRotator` (+ _returnvalue_roll_2 (`self.Speed`)) _returnvalue_pitch_2 _returnvalue_yaw_2) false false)))
            (elif (< _returnvalue_roll_2 -20.0)
              (set `self.ForwardRightLeg` true)
              (else
                (`SceneComponent.K2_SetWorldRotation` _rootleftleg (`KismetMathLibrary.MakeRotator` (- _returnvalue_roll_2 (`self.Speed`)) _returnvalue_pitch_2 _returnvalue_yaw_2) false false)))))
        (:`then_2`
          ;[1 1 1] LeftArm Movement
          (if (`self.ForwardLeftArm`)
            (if (> _returnvalue_roll_3 20.0)
              (set `self.ForwardLeftArm` false)
              (else
                (`SceneComponent.K2_SetWorldRotation` _rootleftarm (`KismetMathLibrary.MakeRotator` (+ _returnvalue_roll_3 (`self.LeftArmSpeed`)) _returnvalue_pitch_3 _returnvalue_yaw_3) false false)))
            (elif (< _returnvalue_roll_3 -20.0)
              (set `self.ForwardLeftArm` true)
              (else
                (`SceneComponent.K2_SetWorldRotation` _rootleftarm (`KismetMathLibrary.MakeRotator` (- _returnvalue_roll_3 (`self.LeftArmSpeed`)) _returnvalue_pitch_3 _returnvalue_yaw_3) false false)))))
        (:`then_3`
          ;[1 1 1] RightArm Movement
          (if (`self.ForwardRightArm`)
            (if (> _returnvalue_roll_4 20.0)
              (set `self.ForwardRightArm` false)
              (else
                (`SceneComponent.K2_SetWorldRotation` _rootrightarm (`KismetMathLibrary.MakeRotator` (+ _returnvalue_roll_4 (`self.RightArmSpeed`)) _returnvalue_pitch_4 _returnvalue_yaw_4) false false)))
            (elif (< _returnvalue_roll_4 -20.0)
              (set `self.ForwardRightArm` true)
              (else
                (`SceneComponent.K2_SetWorldRotation` _rootrightarm (`KismetMathLibrary.MakeRotator` (- _returnvalue_roll_4 (`self.RightArmSpeed`)) _returnvalue_pitch_4 _returnvalue_yaw_4) false false)))))
        (:`then_4`
          ;[1 1 1] Head Movement
          (if (`self.ForwardHead`)
            (if (> _returnvalue_yaw_5 20.0)
              (set `self.ForwardHead` false)
              (else
                (`SceneComponent.K2_SetWorldRotation` _head (`KismetMathLibrary.MakeRotator` _returnvalue_roll_5 _returnvalue_pitch_5 (+ _returnvalue_yaw_5 (`self.HeadSpeed`))) false false)))
            (elif (< _returnvalue_yaw_5 -20.0)
              (set `self.ForwardHead` true)
              (else
                (`SceneComponent.K2_SetWorldRotation` _head (`KismetMathLibrary.MakeRotator` _returnvalue_roll_5 _returnvalue_pitch_5 (- _returnvalue_yaw_5 (`self.HeadSpeed`))) false false)))))))))

(event `self.ReceiveBeginPlay`
  ;[1 1 1] BeginPlay: Sets all limbs to either start moving forward or backward
  (set `self.ForwardLeftLeg` true)
  (set `self.ForwardRightLeg` false)
  (set `self.ForwardLeftArm` true)
  (set `self.ForwardRightArm` false)
  (set `self.ForwardHead` true))

(event `OpenGate`
  ;[1 1 1] EventTick: Gate can be accessed via Events (In the actual case our UI) to stop/continue the animation - Rotates limbs
  (goto _label :!via `Open`))

(event `CloseGate`
  ;[1 1 1] EventTick: Gate can be accessed via Events (In the actual case our UI) to stop/continue the animation - Rotates limbs
  (goto _label :!via `Close`))

(event `Head Slider Changed`
  (params (HeadSpeed :type "Float (double-precision)"))
  ;[1 1 1] On Slider Changed: Sets the resepective value for every slider changed
  (set `self.HeadSpeed` HeadSpeed))

(event `LeftArm Slider Changed`
  (params (LeftArmSpeed :type "Float (double-precision)"))
  ;[1 1 1] On Slider Changed: Sets the resepective value for every slider changed
  (set `self.LeftArmSpeed` LeftArmSpeed))

(event `RightArm Slider Changed`
  (params (RightArmSpeed :type "Float (double-precision)"))
  ;[1 1 1] On Slider Changed: Sets the resepective value for every slider changed
  (set `self.RightArmSpeed` RightArmSpeed))

(fn `UserConstructionScript`)