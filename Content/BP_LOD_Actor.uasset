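; Actor that does custom screen-size LOD, swapping its static mesh between high, medium and low meshes.
; On Tick it projects the eight bounding box corners through the first PlayerController to build a 2D screen extent.
; X and Y sizes, computed as min minus max (so normally negative), are compared against two thresholds to pick the mesh.
; It prints both sizes for debugging and resets its DoOnce after each pass.
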(event `self.ReceiveTick`
  (params (DeltaSeconds :type "Float (single-precision)"))
  (bind (_returnvalue_x _returnvalue_y) (`KismetMathLibrary.BreakVector2D` (`WidgetLayoutLibrary.GetViewportSize`)))
  (bind _hightomediumthreshold (`self.HighToMediumThreshold`))
  (bind (_box_extent_x _box_extent_y _box_extent_z) (`KismetMathLibrary.BreakVector` (`self.Box Extent`)))
  (bind (_box_extent_x_2 _box_extent_y_2 _box_extent_z_2) (`KismetMathLibrary.BreakVector` (`self.Box Extent`)))
  (bind _mediumtolowthreshold (`self.MediumToLowThreshold`))
  (bind (_box_extent_x_3 _box_extent_y_3 _box_extent_z_3) (`KismetMathLibrary.BreakVector` (`self.Box Extent`)))
  (bind (_box_extent_x_4 _box_extent_y_4 _box_extent_z_4) (`KismetMathLibrary.BreakVector` (`self.Box Extent`)))
  (bind (_box_extent_x_5 _box_extent_y_5 _box_extent_z_5) (`KismetMathLibrary.BreakVector` (`self.Box Extent`)))
  (bind (_box_extent_x_6 _box_extent_y_6 _box_extent_z_6) (`KismetMathLibrary.BreakVector` (`self.Box Extent`)))
  (bind _xsize (`self.XSize`))
  (bind _playercontroller (`self.PLayerController`))
  (bind _ysize (`self.YSize`))
  (bind (_origin _boxextent) (`KismetSystemLibrary.GetComponentBounds` (`self.StaticMeshComponent`)))
  (bind _screenposition (`GameplayStatics.ProjectWorldToScreen` _playercontroller (- _origin _boxextent)))
  (bind _screenposition_2 (`GameplayStatics.ProjectWorldToScreen` _playercontroller (+ _origin _boxextent)))
  (`/Engine/EditorBlueprintResources/StandardMacros.DoOnce` false :!label _label
    (:`Completed`
      (if (not false)
        ;[1 1 1] Setup for each Calculation
        (bind _outactors (`GameplayStatics.GetAllActorsOfClass` "/Script/Engine.PlayerController"))
        (set `self.PLayerController` (`|GetArrayItem` _outactors))
        (set `self.MeshOrigin` _origin)
        (set `self.Box Extent` _boxextent)
        (set `self.MaxXPosition` (`KismetMathLibrary.BreakVector2D` _screenposition_2))
        (set `self.MaxYPosition` (`.Y` (`KismetMathLibrary.BreakVector2D` _screenposition_2)))
        (set `self.MinXPosition` (`KismetMathLibrary.BreakVector2D` _screenposition))
        (set `self.MinYPosition` (`.Y` (`KismetMathLibrary.BreakVector2D` _screenposition)))
        (for _array_element (`|MakeArray` (+ (`self.MeshOrigin`) (`self.Box Extent`)) (+ (`self.MeshOrigin`) (`KismetMathLibrary.MakeVector` _box_extent_x_2 _box_extent_y_2 (* _box_extent_z_2 -1.0))) (+ (`self.MeshOrigin`) (`KismetMathLibrary.MakeVector` _box_extent_x_3 (* _box_extent_y_3 -1.0) _box_extent_z_3)) (+ (`self.MeshOrigin`) (`KismetMathLibrary.MakeVector` _box_extent_x_4 (* _box_extent_y_4 -1.0) (* _box_extent_z_4 -1.0))) (+ (`self.MeshOrigin`) (`KismetMathLibrary.MakeVector` (* _box_extent_x_5 -1.0) _box_extent_y_5 _box_extent_z_5)) (+ (`self.MeshOrigin`) (`KismetMathLibrary.MakeVector` (* _box_extent_x_6 -1.0) _box_extent_y_6 (* _box_extent_z_6 -1.0))) (+ (`self.MeshOrigin`) (`KismetMathLibrary.MakeVector` (* _box_extent_x -1.0) (* _box_extent_y -1.0) _box_extent_z)) (- (`self.MeshOrigin`) (`self.Box Extent`)))
          (`|ExecutionSequence`
            (:`then_0`
              (bind (_returnvalue_x_2 _returnvalue_y_2) (`KismetMathLibrary.BreakVector2D` (`KismetMathLibrary.ClampAxes2D` (`GameplayStatics.ProjectWorldToScreen` (`self.PLayerController`) _array_element) _returnvalue_x _returnvalue_y)))
              (if (> _returnvalue_x_2 (`self.MaxXPosition`))
                (set `self.MaxXPosition` _returnvalue_x_2)
                (elif (> (`self.MinXPosition`) _returnvalue_x_2)
                  (set `self.MinXPosition` _returnvalue_x_2))))
            (:`then_1`
              (if (> _returnvalue_y_2 (`self.MaxYPosition`))
                (set `self.MaxYPosition` _returnvalue_y_2)
                (elif (> (`self.MinYPosition`) _returnvalue_y_2)
                  (set `self.MinYPosition` _returnvalue_y_2))))))
        (set `self.XSize` (- (`self.MinXPosition`) (`self.MaxXPosition`)))
        (set `self.YSize` (- (`self.MinYPosition`) (`self.MaxYPosition`)))
        (`|ExecutionSequence`
          (:`then_0`
            (`KismetSystemLibrary.PrintString` (`KismetStringLibrary.Conv_DoubleToString` _xsize))
            (`KismetSystemLibrary.PrintString` (`KismetStringLibrary.Conv_DoubleToString` _ysize))
            (if (or (< _xsize _hightomediumthreshold) (< _ysize _hightomediumthreshold))
              (`StaticMeshComponent.SetStaticMesh` (`self.StaticMeshComponent`) (`self.LODMeshMedium`))
              (elif (or (< _xsize _mediumtolowthreshold) (< _ysize _mediumtolowthreshold))
                (`StaticMeshComponent.SetStaticMesh` (`self.StaticMeshComponent`) (`self.LODMeshLow`))
                (else
                  (`StaticMeshComponent.SetStaticMesh` (`self.StaticMeshComponent`) (`self.LODMeshHigh`))))))
          (:`then_1`
            (`self.ResetTick`)))))))

(event `ResetTick`
  (goto _label :!via `Reset`))

(fn `UserConstructionScript`)