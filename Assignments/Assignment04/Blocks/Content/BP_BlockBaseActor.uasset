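; BP_BlockBaseActor is a block actor that highlights itself while a VRPawn overlaps it.
; Begin and end overlap events on BlockBaseComponent filter for an exact VRPawn class match, then swap material element 0 between M_Highlight_Inst and Default.
; Tick and the construction script are empty, so the behavior is purely event-driven.
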(event `self.BlockBaseComponent.OnComponentEndOverlap`
  (params (OverlappedComponent :type "PrimitiveComponent Object Reference") (OtherActor :type "Actor Object Reference") (OtherComp :type "PrimitiveComponent Object Reference") (OtherBodyIndex :type Integer))
  (if (== (`GameplayStatics.GetObjectClass` OtherActor) "/Game/VRTemplate/Blueprints/VRPawn.VRPawn_C")
    (`PrimitiveComponent.SetMaterial` (`self.BlockBaseComponent`) 0 "/Game/Blocks/Meshes/default.default")))

(event `self.BlockBaseComponent.OnComponentBeginOverlap`
  (params (OverlappedComponent :type "PrimitiveComponent Object Reference") (OtherActor :type "Actor Object Reference") (OtherComp :type "PrimitiveComponent Object Reference") (OtherBodyIndex :type Integer) (bFromSweep :type Boolean) (SweepResult :type "HitResult Structure (by ref)"))
  (if (== (`GameplayStatics.GetObjectClass` OtherActor) "/Game/VRTemplate/Blueprints/VRPawn.VRPawn_C")
    (`PrimitiveComponent.SetMaterial` (`self.BlockBaseComponent`) 0 "/Game/Materials/M_Highlight_Inst.M_Highlight_Inst")))

(fn `UserConstructionScript`)