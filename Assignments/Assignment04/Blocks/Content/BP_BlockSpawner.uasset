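; BP_BlockSpawner is an actor that keeps a supply of blocks at its location.
; On BeginPlay it spawns one actor of its BlockType class at its root transform.
; When an actor of exactly that class stops overlapping its Box, it spawns another at the same transform, so a replacement appears each time a block leaves.
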(event `self.ReceiveBeginPlay`
  (`|SpawnActorFromClass` (`self.BlockType`) (`SceneComponent.K2_GetComponentToWorld` (`self.DefaultSceneRoot`)) "Undefined" "MultiplyWithRoot" null null))

(event `self.Box.OnComponentEndOverlap`
  (params (OverlappedComponent :type "PrimitiveComponent Object Reference") (OtherActor :type "Actor Object Reference") (OtherComp :type "PrimitiveComponent Object Reference") (OtherBodyIndex :type Integer))
  (bind _blocktype (`self.BlockType`))
  (if (== (`GameplayStatics.GetObjectClass` OtherActor) _blocktype)
    (`|SpawnActorFromClass` _blocktype (`SceneComponent.K2_GetComponentToWorld` (`self.DefaultSceneRoot`)) "Undefined" "MultiplyWithRoot" null null)))

(fn `UserConstructionScript`)